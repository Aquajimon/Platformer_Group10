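; BP_FollowCam is a side-scroller camera actor that follows BP_SideScrollerCharacter at an offset, never moving back along X.
; The construction script places it at the character plus offset, and SetCamera caches the player and starting location.
; Each Tick follows the player, clamps Z to that starting height, then PoNREvent holds X at the furthest point reached.
; Without a valid player, it returns to the stored location and retries SetCamera.
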(event Custom|PoNR%20Event
  (bind _returnvalue (Transformation|GetActorLocation))
  (if (> (Variables|Default|GetSideLock) (.x (Variables|Default|GetCameraPosition)))
    _
    (else
      (Variables|Default|SetSideLock (.x _returnvalue))))
  (Transformation|SetActorLocation (Math|Vector|MakeVector (Variables|Default|GetSideLock) (.y _returnvalue) (.z _returnvalue)) false false))

(event Custom|Set%20Camera
  ;[0.15 0.15 0.15 0.5] Store Ref. to the player object
  (bind _asbp_side_scroller_character (Utilities|Casting|CastToBP_SideScrollerCharacter (Game|GetPlayerCharacter 0)))
  (Variables|Default|SetPlayerRef _asbp_side_scroller_character)
  (bind _output_get (Variables|Default|SetLowestHeight (Transformation|GetActorLocation)))
  (Variables|Default|SetSideLock (.x _output_get)))

(event EventBeginPlay
  (CallFunction|SetCamera))

(event EventTick
  (params (DeltaSeconds :type Float%20%28single-precision%29))
  (bind _offset (Variables|Default|GetOffset))
  (bind _playerref (Variables|Default|GetPlayerRef))
  (bind _returnvalue (Transformation|GetActorLocation _playerref))
  (bind _returnvalue_2 (+ _returnvalue _offset))
  ;[0.15 0.15 0.15 0.5] Set Camera at players position w/ offset
  (Utilities|IsValid _playerref
    (:Is%20Valid
      (bind _output_get (Variables|Default|SetCameraPosition _returnvalue_2))
      (if (< (.z (Variables|Default|GetCameraPosition)) (.z (Variables|Default|GetLowestHeight)))
        (Transformation|SetActorLocation (Math|Vector|MakeVector (.x _output_get) (.y _output_get) (.z (Variables|Default|GetLowestHeight))) false false)
        (CallFunction|PoNREvent)
        (else
          (Transformation|SetActorLocation _returnvalue_2 false false)
          (CallFunction|PoNREvent))))
    (:Is%20Not%20Valid
      (Transformation|SetActorLocation (Variables|Default|GetLowestHeight) false false)
      (CallFunction|SetCamera))))

(fn ConstructionScript
  (bind _returnvalue (Actor|GetActorOfClass "/Game/Blueprints/BP_SideScrollerCharacter.BP_SideScrollerCharacter_C"))
  (Transformation|SetActorLocation (+ (Transformation|GetActorLocation _returnvalue) (Variables|Default|GetOffset)) true false))