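; BP_StarBlock is a block that spawns a bouncing invincibility star power-up when the side-scroller character overlaps it.
; On overlap it spawns BP_InvincibleStar at the SpawnItem component's location and gives it a default controller, with no guard against repeat spawns.
; The construction script creates a dynamic material on the Block component and tints it with the BlockColor variable.
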(event Collision|EventActorBeginOverlap
  (params (OtherActor :type Actor%20Object%20Reference))
  ;[0.15 0.15 0.15 0.5] Spawns Bouncing star power-up once character hits block
  (Utilities|Casting|CastToBP_SideScrollerCharacter OtherActor)
  (bind _returnvalue (Game|SpawnActorfromClass "/Game/Blueprints/AdrianWork/Collectables/BP_InvincibleStar.BP_InvincibleStar_C" (Math|Transform|MakeTransform (Transformation|GetWorldLocation (Variables|Default|GetSpawnItem)) "0, 0, 0" "1.000000,1.000000,1.000000") "Undefined" "MultiplyWithRoot" 0 0))
  (Utilities|IsValid _returnvalue
    (:Is%20Valid
      (Pawn|SpawnDefaultController _returnvalue))))

(fn ConstructionScript
  (bind _returnvalue (Rendering|Material|CreateDynamicMaterialInstance (Variables|Default|GetBlock) 0 0 "None" :!class /Script/Engine.PrimitiveComponent))
  (Rendering|Material|SetVectorParameterValue _returnvalue "Color" (Variables|Default|GetBlockColor) :!class /Script/Engine.MaterialInstanceDynamic))