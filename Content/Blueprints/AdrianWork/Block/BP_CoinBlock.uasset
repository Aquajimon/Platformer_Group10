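; BP_CoinBlock is a block that releases a single gold coin for the side-scroller character.
; On its first actor overlap, it casts the other actor to BP_SideScrollerCharacter and spawns a BP_GoldCoin at the SpawnItem component's world location.
; The DoOnce gate sits before the cast, so any overlapping actor consumes the one use, even if no coin spawns.
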(event EventBeginPlay
  (|CallParentFunction) ; This node is disabled and will not be called.\nDrag off pins to build functionality.
)

(event Collision|EventActorBeginOverlap
  (params (OtherActor :type Actor%20Object%20Reference))
  (Utilities|FlowControl|DoOnce false
    (:Completed
      (Utilities|Casting|CastToBP_SideScrollerCharacter OtherActor)
      (Game|SpawnActorfromClass "/Game/Blueprints/AdrianWork/Collectables/BP_GoldCoin.BP_GoldCoin_C" (Math|Transform|MakeTransform (Transformation|GetWorldLocation (Variables|Default|GetSpawnItem)) "0, 0, 0" "1.000000,1.000000,1.000000") "Undefined" "MultiplyWithRoot" 0 0))))

(event EventTick
  (params (DeltaSeconds :type Float%20%28single-precision%29))
  (|CallParentFunction DeltaSeconds) ; This node is disabled and will not be called.\nDrag off pins to build functionality.
)

(fn ConstructionScript
  (|CallParentFunction))