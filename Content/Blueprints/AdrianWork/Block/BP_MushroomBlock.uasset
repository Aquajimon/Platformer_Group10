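; BP_MushroomBlock is a block that spawns a mushroom when the side-scroller player character overlaps it.
; On ActorBeginOverlap it casts to BP_SideScrollerCharacter, spawns BP_MushroomNEW at the SpawnItem component's world location, then calls SpawnDefaultController on the new mushroom.
; The overlap has no one-shot guard, so each new player overlap spawns another mushroom.
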(event EventBeginPlay
  (|CallParentFunction) ; This node is disabled and will not be called.\nDrag off pins to build functionality.
)

(event Collision|EventActorBeginOverlap
  (params (OtherActor :type Actor%20Object%20Reference))
  (Utilities|Casting|CastToBP_SideScrollerCharacter OtherActor)
  (bind _returnvalue (Game|SpawnActorfromClass "/Game/Blueprints/AdrianWork/Collectables/BP_MushroomNEW.BP_MushroomNEW_C" (Math|Transform|MakeTransform (Transformation|GetWorldLocation (Variables|Default|GetSpawnItem)) "0, 0, 0" "1.000000,1.000000,1.000000") "Undefined" "MultiplyWithRoot" 0 0))
  (Pawn|SpawnDefaultController _returnvalue))

(event EventTick
  (params (DeltaSeconds :type Float%20%28single-precision%29))
  (|CallParentFunction DeltaSeconds) ; This node is disabled and will not be called.\nDrag off pins to build functionality.
)

(fn ConstructionScript
  (|CallParentFunction))