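; BP_FAILEDMushroom is a moving pickup that makes the side-scroller character grow on overlap, then removes itself.
; Tick sweeps the static mesh by MoveSpeed along MoveDir each frame, without delta-time scaling.
; Any Hit event toggles MoveDir between positive and negative X via a FlipFlop.
; The overlap Sequence stores PlayerRef and calls DestroyActor before MushroomGrow runs, then reaches the same destroy again.
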(event OnComponentBeginOverlap(StaticMesh)
  (params (OverlappedComponent :type Primitive%20Component%20Object%20Reference) (OtherActor :type Actor%20Object%20Reference) (OtherComp :type Primitive%20Component%20Object%20Reference) (OtherBodyIndex :type Integer) (bFromSweep :type Boolean) (SweepResult :type Hit%20Result%20Structure%20%28by%20ref%29))
  ;[0.15 0.15 0.15 0.5] Mushroom can be picked up and cause player to grow, destroying itself afterwards
  (bind _asbp_side_scroller_character (Utilities|Casting|CastToBP_SideScrollerCharacter OtherActor))
  (Utilities|FlowControl|Sequence
    (:then_0
      (Variables|Default|SetPlayerRef _asbp_side_scroller_character))
    (:then_1
      (Default|MushroomGrow _asbp_side_scroller_character)))
  (Actor|DestroyActor))

(event EventBeginPlay)

(event Collision|EventActorBeginOverlap
  (params (OtherActor :type Actor%20Object%20Reference)))

(event EventTick
  (params (DeltaSeconds :type Float%20%28single-precision%29))
  ;[0.15 0.15 0.15 0.5] Move Mushroom
  (Utilities|FlowControl|Sequence
    (:then_0
      (Transformation|AddWorldOffset (Variables|Default|GetStaticMesh) (* (Variables|Default|GetMoveSpeed) (Variables|Default|GetMoveDir)) true false))))

(event Collision|EventHit
  (params (MyComp :type Primitive%20Component%20Object%20Reference) (Other :type Actor%20Object%20Reference) (OtherComp :type Primitive%20Component%20Object%20Reference) (bSelfMoved :type Boolean) (HitLocation :type Vector :default "0, 0, 0") (HitNormal :type Vector :default "0, 0, 0") (NormalImpulse :type Vector :default "0, 0, 0") (Hit :type Hit%20Result%20Structure%20%28by%20ref%29))
  ;[0.15 0.15 0.15 0.5] Mushroom goes opposite direction when hitting a wall
  (Utilities|FlowControl|FlipFlop
    (:A
      (Variables|Default|SetMoveDir "1.000000,0.000000,0.000000"))
    (:B
      (Variables|Default|SetMoveDir "-1.000000,0.000000,0.000000"))))

(fn ConstructionScript)