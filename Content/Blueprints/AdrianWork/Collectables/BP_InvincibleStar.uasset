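; Invincibility star pickup that moves and bounces on its own, granting star power to the side-scroller character.
; Every Tick it applies half-scale movement input along MoveDir and calls Jump.
; Each Hit event alternates MoveDir's X sign through a FlipFlop, intended to reverse it at walls.
; Capsule overlap with BP_SideScrollerCharacter stores the player reference, calls StarPower on it and destroys the star.
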(event OnComponentBeginOverlap(CapsuleComponent)
  (params (OverlappedComponent :type Primitive%20Component%20Object%20Reference) (OtherActor :type Actor%20Object%20Reference) (OtherComp :type Primitive%20Component%20Object%20Reference) (OtherBodyIndex :type Integer) (bFromSweep :type Boolean) (SweepResult :type Hit%20Result%20Structure%20%28by%20ref%29))
  ;[0.15 0.15 0.15 0.5] Character collects star, then becomes invincible, destroying star
  (bind _asbp_side_scroller_character (Utilities|Casting|CastToBP_SideScrollerCharacter OtherActor))
  (Utilities|FlowControl|Sequence
    (:then_0
      (Variables|Default|SetPlayerRef _asbp_side_scroller_character))
    (:then_1
      (Default|StarPower _asbp_side_scroller_character)))
  (Actor|DestroyActor))

(event EventBeginPlay)

(event Collision|EventActorBeginOverlap
  (params (OtherActor :type Actor%20Object%20Reference)))

(event EventTick
  (params (DeltaSeconds :type Float%20%28single-precision%29))
  ;[0.15 0.15 0.15 0.5] Movement
  (Pawn|Input|AddMovementInput (Variables|Default|GetMoveDir) 0.5 false)
  (Character|Jump))

(event Collision|EventHit
  (params (MyComp :type Primitive%20Component%20Object%20Reference) (Other :type Actor%20Object%20Reference) (OtherComp :type Primitive%20Component%20Object%20Reference) (bSelfMoved :type Boolean) (HitLocation :type Vector :default "0, 0, 0") (HitNormal :type Vector :default "0, 0, 0") (NormalImpulse :type Vector :default "0, 0, 0") (Hit :type Hit%20Result%20Structure%20%28by%20ref%29))
  ;[0.15 0.15 0.15 0.5] Move opposite direction when hitting walls
  (Utilities|FlowControl|FlipFlop
    (:A
      (Variables|Default|SetMoveDir "1.000000,0.000000,1.000000"))
    (:B
      (Variables|Default|SetMoveDir "-1.000000,0.000000,1.000000"))))

(fn ConstructionScript)