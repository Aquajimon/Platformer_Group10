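; Base pickup actor for the side-scroller that triggers when the player character overlaps it, then destroys itself.
; On overlap it casts to BP_SideScrollerCharacter, stores the player reference and calls OnPickup before destruction.
; OnPickup plays the pickup sound at the actor's location, or prints a message if none is set.
; The construction script applies an adjustable Color to a dynamic M_Metallic material instance on the mesh.
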(event Custom|OnPickup
  ;[1 0 0 0.5] Play sound on pickup
  (bind _pickupsfx (Variables|Default|GetPickupSFX)
    (:then
      (Audio|PlaySoundatLocation _pickupsfx (Transformation|GetActorLocation) "0, 0, 0" 1.0 1.0 0.0 0 0 0 0))
    (:else
      (Development|PrintString "No SFX Set"))))

(event Collision|EventActorBeginOverlap
  (params (OtherActor :type Actor%20Object%20Reference))
  ;[0 0 0] Pick Up on Overlap
  (bind _asbp_side_scroller_character (Utilities|Casting|CastToBP_SideScrollerCharacter OtherActor))
  (Variables|Default|SetPlayerRef _asbp_side_scroller_character)
  (CallFunction|OnPickup)
  (Actor|DestroyActor))

(fn ConstructionScript
  ;[0 0 0] Set Adjustable Color Parameter
  (bind _returnvalue (Rendering|Material|CreateDynamicMaterialInstance (Variables|Default|GetStaticMesh) 0 "/Game/Materials/M_Metallic.M_Metallic" "None" :!class /Script/Engine.PrimitiveComponent))
  (Rendering|Material|SetVectorParameterValue _returnvalue "Color" (Variables|Default|GetColor) :!class /Script/Engine.MaterialInstanceDynamic))