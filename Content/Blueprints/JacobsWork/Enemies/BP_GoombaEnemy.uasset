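; BP_GoombaEnemy is a Goomba enemy that simulates basic gravity through its MoveDirection vector.
; A GroundDetection overlap caches the last BP_Enviornment actor it began touching.
; After calling the parent Tick, it sets MoveDirection Z to zero while overlapping that cached actor and to a constant downward value otherwise, leaving X and Y unchanged.
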(event OnComponentBeginOverlap(GroundDetection)
  (params (OverlappedComponent :type Primitive%20Component%20Object%20Reference) (OtherActor :type Actor%20Object%20Reference) (OtherComp :type Primitive%20Component%20Object%20Reference) (OtherBodyIndex :type Integer) (bFromSweep :type Boolean) (SweepResult :type Hit%20Result%20Structure%20%28by%20ref%29))
  ;[0.15 0.15 0.15 0.5] Simulates Basic Gravity for the Goomba
  (bind _asbp_enviornment (Utilities|Casting|CastToBP_Enviornment OtherActor)))

(event EventTick
  (params (DeltaSeconds :type Float%20%28single-precision%29))
  ;[0.15 0.15 0.15 0.5] Simulates Basic Gravity for the Goomba
  (|CallParentFunction DeltaSeconds)
  (if (Collision|IsOverlappingActor (Variables|Default|GetGround%20Detection) (stale OnComponentBeginOverlap(GroundDetection) _asbp_enviornment) :!class /Script/Engine.PrimitiveComponent)
    (Variables|Default|SetMoveDirection (Math|Vector|MakeVector (.x (Variables|Default|GetMoveDirection)) (.y (Variables|Default|GetMoveDirection)) 0.0))
    (else
      (Variables|Default|SetMoveDirection (Math|Vector|MakeVector (.x (Variables|Default|GetMoveDirection)) (.y (Variables|Default|GetMoveDirection)) -1.0)))))

(fn ConstructionScript
  (|CallParentFunction))