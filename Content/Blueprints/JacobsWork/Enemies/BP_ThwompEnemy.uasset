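; Thwomp-style enemy that drops, then rises slowly back to the home position saved at BeginPlay.
; Tick manages CanMove from home position and player-area state, and treats any nonzero HitNormal.Z while away from home as ground contact.
; The return event waits, raises the thwomp through EnemyMove, snaps it home, then restores downward movement after another delay.
; The construction script tints the cube dark grey-green.
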(event Custom|ThwompTheWayHome
  ;[0.15 0.15 0.15 0.5] Moves the thwomp back to it's original position
  (if (Variables|Default|GetWait%20time)
    (Variables|Default|SetMoveDirection "0.000000,0.000000,0.250000")
    (CallFunction|EnemyMove)
    ;[0.15 0.15 0.15 0.5] Resets the Thwomp
    (if (>= (.z (Transformation|GetActorLocation)) (.z (Variables|Default|GetThwompHome)))
      (Variables|Default|SetMoveDirection "0, 0, 0")
      (Variables|Default|SetHit%20Normal "0, 0, 0")
      (Transformation|SetActorLocation (Variables|Default|GetThwompHome) true false)
      (Utilities|FlowControl|Delay 2.0)
      (Variables|Default|SetMoveDirection "0.000000,0.000000,-1.000000")
      (Variables|Default|SetWait%20time false))
    (else
      (Utilities|FlowControl|Delay 2.0)
      (Variables|Default|SetWait%20time true))))

(event EventBeginPlay
  ;[0.15 0.15 0.15 0.5] Sets the thwomps home to begining placement
  (|CallParentFunction)
  (Variables|Default|SetThwompHome (Transformation|GetActorLocation)))

(event EventTick
  (params (DeltaSeconds :type Float%20%28single-precision%29))
  (bind _hit_normal (Variables|Default|GetHit%20Normal))
  ;[0.15 0.15 0.15 0.5] Detects whether thwomp has hit the ground, if so, calls for it to return to home point
  (|CallParentFunction DeltaSeconds)
  (if (Utilities|Operators|EqualEqual (Transformation|GetActorLocation) (Variables|Default|GetThwompHome) 0.0)
    (Variables|Default|SetCanMove false)
    (else
      (if (Variables|Default|GetIsPlayerInArea)
        _
        (else
          (Variables|Default|SetCanMove true)))
      (if (>= (/ (.z _hit_normal) (.z _hit_normal)) 1.0)
        (CallFunction|ThwomptheWayHome)))))

(fn ConstructionScript
  (|CallParentFunction)
  (Rendering|Material|SetColorParameterValueonMaterials (Variables|Default|GetCube) "Color" "(R=0.137369,G=0.194792,B=0.170993,A=1.000000)"))