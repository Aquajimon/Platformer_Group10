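; Temporary end-of-level flag that advances the side-scroller to the next level when the player character reaches it.
; A one-shot Box overlap sets FlagFall and calls NextLevel on the game instance cached at BeginPlay, while a character hit on the Base clears FlagFall.
; The construction script tints the base, flag and pole materials.
; Tick is empty, and the logic to move the character and flag is disconnected, so it never runs.
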(event OnComponentBeginOverlap(Box)
  (params (OverlappedComponent :type Primitive%20Component%20Object%20Reference) (OtherActor :type Actor%20Object%20Reference) (OtherComp :type Primitive%20Component%20Object%20Reference) (OtherBodyIndex :type Integer) (bFromSweep :type Boolean) (SweepResult :type Hit%20Result%20Structure%20%28by%20ref%29))
  (Utilities|FlowControl|DoOnce false
    (:Completed
      (bind _asbp_side_scroller_character (Utilities|Casting|CastToBP_SideScrollerCharacter OtherActor))
      (Variables|Default|SetFlagFall true)
      (Default|NextLevel (stale EventBeginPlay _output_get)))))

(event OnComponentHit(Base)
  (params (HitComponent :type Primitive%20Component%20Object%20Reference) (OtherActor :type Actor%20Object%20Reference) (OtherComp :type Primitive%20Component%20Object%20Reference) (NormalImpulse :type Vector :default "0, 0, 0") (Hit :type Hit%20Result%20Structure%20%28by%20ref%29))
  (Utilities|Casting|CastToBP_SideScrollerCharacter OtherActor)
  (Variables|Default|SetFlagFall false))

(event EventBeginPlay
  (bind _asbp_game_instance (Utilities|Casting|CastToBP_GameInstance (Game|GetGameInstance)))
  (bind _output_get (Variables|Default|SetAs%20BP%20Game%20Instance _asbp_game_instance)))

(event EventTick
  (params (DeltaSeconds :type Float%20%28single-precision%29)))

(fn ConstructionScript
  (Rendering|Material|SetColorParameterValueonMaterials (Variables|Default|GetBase) "Color" "(R=0.223958,G=0.088064,B=0.031961,A=1.000000)")
  (Rendering|Material|SetColorParameterValueonMaterials (Variables|Default|GetFlag) "Color" "(R=1.000000,G=1.000000,B=1.000000,A=1.000000)")
  (Rendering|Material|SetColorParameterValueonMaterials (Variables|Default|GetFlagPole) "Color" "(R=0.000000,G=0.290625,B=0.027645,A=1.000000)"))