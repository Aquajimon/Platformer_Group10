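; BP_tempCheckpoint is a side-scroller checkpoint with a flag, pole and overlap box that moves the level's respawn point.
; When BP_SideScrollerCharacter overlaps the box, it finds the BP_Respawn actor and moves it to the checkpoint's X and Z, keeping its own Y.
; The flag then turns red through a material color parameter.
; The construction script sets the starting brown cylinder and black flag colors.
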(event OnComponentBeginOverlap(Box)
  (params (OverlappedComponent :type Primitive%20Component%20Object%20Reference) (OtherActor :type Actor%20Object%20Reference) (OtherComp :type Primitive%20Component%20Object%20Reference) (OtherBodyIndex :type Integer) (bFromSweep :type Boolean) (SweepResult :type Hit%20Result%20Structure%20%28by%20ref%29))
  (bind _returnvalue (Transformation|GetActorLocation))
  (Utilities|Casting|CastToBP_SideScrollerCharacter OtherActor)
  (bind _returnvalue_2 (Actor|GetActorOfClass "/Game/Blueprints/JuanWork/LevelStuff/BP_Respawn.BP_Respawn_C"))
  (Transformation|SetActorLocation _returnvalue_2 (Math|Vector|MakeVector (.x _returnvalue) (.y (Transformation|GetActorLocation _returnvalue_2)) (.z _returnvalue)) false false)
  (Rendering|Material|SetColorParameterValueonMaterials (Variables|Default|GetFlag) "Color" "(R=0.973958,G=0.000000,B=0.028708,A=1.000000)"))

(fn ConstructionScript
  (Rendering|Material|SetColorParameterValueonMaterials (Variables|Default|GetCylinder) "Color" "(R=0.173958,G=0.070139,B=0.030624,A=1.000000)")
  (Rendering|Material|SetColorParameterValueonMaterials (Variables|Default|GetFlag) "Color" "(R=0.000000,G=0.000000,B=0.000000,A=1.000000)"))