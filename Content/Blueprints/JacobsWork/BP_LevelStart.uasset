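; BP_LevelStart is a level start actor that shows a widget and pins the side-scroller player character at its own location.
; On BeginPlay it caches the player pawn, adds the widget to the viewport, then clears the GameStart flag after a two-second delay.
; While GameStart is true, Tick moves the character to the actor's location every frame without sweeping.
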(event EventBeginPlay
  (bind _asbp_side_scroller_character (Utilities|Casting|CastToBP_SideScrollerCharacter (Game|Player|GetPlayerPawn 0)))
  (bind _returnvalue (UserInterface|CreateWidget (Variables|Default|GetClass)))
  (UserInterface|Viewport|AddtoViewport _returnvalue 0)
  (Utilities|FlowControl|Delay 2.0)
  (Variables|Default|SetGameStart false))

(event EventTick
  (params (DeltaSeconds :type Float%20%28single-precision%29))
  (if (Variables|Default|GetGameStart)
    (Transformation|SetActorLocation (stale EventBeginPlay _asbp_side_scroller_character) (Transformation|GetActorLocation) false false)))

(fn ConstructionScript)